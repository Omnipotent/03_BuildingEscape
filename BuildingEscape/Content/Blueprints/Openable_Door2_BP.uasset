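; Openable door Blueprint that swings open and shut in response to OpenDoor's OnOpen and OnClose events.
; The DoorSwing timeline plays forward or in reverse, adding a yaw angle to the rotation saved at BeginPlay.
; Timeline event tracks trigger the open and close sounds, with a DoOnce gating the close sound until the timeline finishes and resets it.
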(event OnClose(OpenDoor)
  (bind _returnvalue (Transformation|GetActorLocation))
  (bind _open_angle (Timeline|Door%20Swing Reverse)
    (:Update
      (Transformation|SetActorRotation (Math|Rotator|CombineRotators (Math|Rotator|MakeRotator 0.0 0.0 _open_angle) (Variables|Default|GetInitial%20Rotation))))
    (:Finished
      (goto _label Reset))
    (:Door%20Open%20Sound
      (Audio|PlaySoundatLocation "/Game/Audio/door_open_004_16bit.door_open_004_16bit" _returnvalue))
    (:Door%20Close%20Sound
      (Utilities|FlowControl|DoOnce false :!label _label
        (:Completed
          (Audio|PlaySoundatLocation "/Game/Audio/door_close_003_16bit.door_close_003_16bit" _returnvalue))))))

(event OnOpen(OpenDoor)
  (bind _returnvalue (Transformation|GetActorLocation))
  (bind _open_angle (Timeline|Door%20Swing Play)
    (:Update
      (Transformation|SetActorRotation (Math|Rotator|CombineRotators (Math|Rotator|MakeRotator 0.0 0.0 _open_angle) (Variables|Default|GetInitial%20Rotation))))
    (:Finished
      (goto _label Reset))
    (:Door%20Open%20Sound
      (Audio|PlaySoundatLocation "/Game/Audio/door_open_004_16bit.door_open_004_16bit" _returnvalue))
    (:Door%20Close%20Sound
      (Utilities|FlowControl|DoOnce false :!label _label
        (:Completed
          (Audio|PlaySoundatLocation "/Game/Audio/door_close_003_16bit.door_close_003_16bit" _returnvalue))))))

(event EventBeginPlay
  (Variables|Default|SetInitial%20Rotation (Transformation|GetActorRotation)))

(fn ConstructionScript)